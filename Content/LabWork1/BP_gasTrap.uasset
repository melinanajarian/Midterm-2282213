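; Gas trap actor that repeatedly damages the third-person player character while it overlaps the trap.
; On overlap, a character with HaveGasDefuse destroys the trap; otherwise a looping timer starts, with a negative start delay cancelling the first wait.
; Each tick of the timer plays a hit montage on the character and applies DamageAmount damage.
; Ending the overlap pauses the timer.
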(event `self.ReceiveActorBeginOverlap`
  (params (OtherActor :type "Actor Object Reference"))
  (bind _asbp_third_person_character (cast `/Game/ThirdPerson/Blueprints/BP_ThirdPersonCharacter` OtherActor))
  (set `self.As BP Third Person Character` _asbp_third_person_character)
  (if (`/Game/ThirdPerson/Blueprints/BP_ThirdPersonCharacter.haveGasDefuse?` (`self.As BP Third Person Character`))
    (`self.K2_DestroyActor`)
    (else
      (`KismetSystemLibrary.K2_SetTimer` null "damage player" 0.7 true -0.7))))

(event `self.ReceiveActorEndOverlap`
  (params (OtherActor :type "Actor Object Reference"))
  (cast `/Game/ThirdPerson/Blueprints/BP_ThirdPersonCharacter` OtherActor)
  (`KismetSystemLibrary.K2_PauseTimer` null "damage player"))

(event `damage player`
  (`Character.PlayAnimMontage` (`self.As BP Third Person Character`) "/Game/LabWork1/Animations/Hit_To_Body_Montage.Hit_To_Body_Montage" 1.0 "None")
  (`GameplayStatics.ApplyDamage` (`self.As BP Third Person Character`) (`self.damageAmount`)))

(fn `UserConstructionScript`)