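; BP_MazeCell is a modular maze cell actor that builds its own geometry and lighting.
; The construction script scales the floor from GridSize and adds optional walls, a ceiling and a point light, using SizeToCubeScale for cube mesh scales.
; At BeginPlay it binds to the third-person character's maze gate event, recoloring its light to the character's LightColor when that event reports not inside.
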(event `self.ReceiveBeginPlay`
  (bind _asbp_third_person_character (cast `/Game/ThirdPerson/Blueprints/BP_ThirdPersonCharacter` (`GameplayStatics.GetPlayerPawn` 0)))
  (set `self.As BP Third Person Character` _asbp_third_person_character)
  (add `/Game/ThirdPerson/Blueprints/BP_ThirdPersonCharacter.Maze_Gate` _asbp_third_person_character (delegate `MazeGate Event`)))

(event `MazeGate Event`
  (params (`isInside?` :type Boolean))
  (bind _pointlight (`self.PointLight`))
  (if (not `isInside?`)
    (`/Engine/EditorBlueprintResources/StandardMacros.IsValid` _pointlight
      (:`Is Valid`
        (`LightComponent.SetLightColor` _pointlight (`/Game/ThirdPerson/Blueprints/BP_ThirdPersonCharacter.LightColor` (`self.As BP Third Person Character`)) true)))))

(fn `UserConstructionScript`
  (locals (WallLenght :type "Float (double-precision)") (WallThickness :type "Float (double-precision)"))
  (bind _gridsize (`self.GridSize`))
  (bind _walllenght (`local.WallLenght`))
  (bind _walllenght_2 (`local.WallLenght`))
  (bind _returnvalue (* (`local.WallLenght`) 0.5))
  (set `local.WallLenght` _gridsize)
  (set `local.WallThickness` (* _gridsize 0.1))
  (`SceneComponent.SetRelativeScale3D` (`self.Floor`) (`self.SizeToCubeScale` (`KismetMathLibrary.MakeVector` _walllenght _walllenght (`local.WallThickness`))))
  (if (`self.WestWal`)
    (`AddComponent|NODE_AddStaticMeshComponent-0` :`RelativeTransform` (`KismetMathLibrary.MakeTransform` (0.0 0.0 0.0) (struct) (`self.SizeToCubeScale` (`KismetMathLibrary.MakeVector` (`local.WallLenght`) (`local.WallThickness`) (`self.WallHeight`))))))
  (if (`self.SouthWall`)
    (`AddComponent|NODE_AddStaticMeshComponent-1` :`RelativeTransform` (`KismetMathLibrary.MakeTransform` (0.0 0.0 0.0) (struct) (`self.SizeToCubeScale` (`KismetMathLibrary.MakeVector` (`local.WallThickness`) (`local.WallLenght`) (`self.WallHeight`))))))
  (if (`self.NorthWall`)
    (`AddComponent|NODE_AddStaticMeshComponent-2` :`RelativeTransform` (`KismetMathLibrary.MakeTransform` (`KismetMathLibrary.MakeVector` (- (`local.WallLenght`) (`local.WallThickness`))) (struct) (`self.SizeToCubeScale` (`KismetMathLibrary.MakeVector` (`local.WallThickness`) (`local.WallLenght`) (`self.WallHeight`))))))
  (if (`self.EastWall`)
    (`AddComponent|NODE_AddStaticMeshComponent-3` :`RelativeTransform` (`KismetMathLibrary.MakeTransform` (`KismetMathLibrary.MakeVector` 0.0 (- (`local.WallLenght`) (`local.WallThickness`))) (struct) (`self.SizeToCubeScale` (`KismetMathLibrary.MakeVector` (`local.WallLenght`) (`local.WallThickness`) (`self.WallHeight`))))))
  (if (`self.Ceiling`)
    (`AddComponent|NODE_AddStaticMeshComponent-4` :`RelativeTransform` (`KismetMathLibrary.MakeTransform` (`KismetMathLibrary.MakeVector` 0.0 0.0 (`self.WallHeight`)) (struct) (`self.SizeToCubeScale` (`KismetMathLibrary.MakeVector` _walllenght_2 _walllenght_2 (`local.WallThickness`))))))
  (if (> (`self.Light intensity`) 0.0)
    (bind _returnvalue_2 (`AddComponent|NODE_AddPointLightComponent-0` :`RelativeTransform` (`KismetMathLibrary.MakeTransform` (`KismetMathLibrary.MakeVector` _returnvalue _returnvalue (* (`self.WallHeight`) 0.9)))))
    (bind _output_get (set `self.PointLight` _returnvalue_2))
    (`LightComponent.SetLightColor` _output_get (`self.Light color`) true)
    (`LightComponent.SetIntensity` _output_get (`self.Light intensity`))))