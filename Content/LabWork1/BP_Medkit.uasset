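; BP_Medkit is a healing pickup that restores the player character's health when interacted with.
; On BeginPlay it casts and caches the local player's BP_ThirdPersonCharacter.
; Its Interact event adds HealingAmount to that character's Health, caps the result at 100, then destroys the medkit.
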(event `self.ReceiveBeginPlay`
  (bind _asbp_third_person_character (cast `/Game/ThirdPerson/Blueprints/BP_ThirdPersonCharacter` (`GameplayStatics.GetPlayerCharacter` 0)))
  (set `self.As BP Third Person Character` _asbp_third_person_character))

(event `/Game/LabWork1/BPI_Interactable.Interact`
  (bind _as_bp_third_person_character (`self.As BP Third Person Character`))
  (bind _returnvalue (+ (`/Game/ThirdPerson/Blueprints/BP_ThirdPersonCharacter.Health` _as_bp_third_person_character) (`self.healingAmount`)))
  (if (> _returnvalue 100.0)
    (set `/Game/ThirdPerson/Blueprints/BP_ThirdPersonCharacter.Health` 100.0 (`self.As BP Third Person Character`))
    (else
      (set `/Game/ThirdPerson/Blueprints/BP_ThirdPersonCharacter.Health` _returnvalue _as_bp_third_person_character)))
  (`self.K2_DestroyActor`))

(fn `UserConstructionScript`)