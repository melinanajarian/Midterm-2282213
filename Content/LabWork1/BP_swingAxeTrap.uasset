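; Swinging axe trap that damages the third-person character, or destroys itself if the character carries an axe defuse.
; Overlapping trigger R without the defuse starts a looping timer that calls the trap activation event.
; That event runs the Swing timeline through a DoOnce, rotating two meshes back and forth by alternating Play and Reverse.
; A hit from either mesh plays a hit montage on the character and applies damage.
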(event `self.r.OnComponentBeginOverlap`
  (params (OverlappedComponent :type "PrimitiveComponent Object Reference") (OtherActor :type "Actor Object Reference") (OtherComp :type "PrimitiveComponent Object Reference") (OtherBodyIndex :type Integer) (bFromSweep :type Boolean) (SweepResult :type "HitResult Structure (by ref)"))
  (bind _asbp_third_person_character (cast `/Game/ThirdPerson/Blueprints/BP_ThirdPersonCharacter` OtherActor))
  (bind _output_get (set `self.As BP Third Person Character` _asbp_third_person_character))
  (if (`/Game/ThirdPerson/Blueprints/BP_ThirdPersonCharacter.haveAxeDefuse?` _output_get)
    (`KismetSystemLibrary.K2_PauseTimer` null "active trap")
    (`self.K2_DestroyActor`)
    (else
      (`KismetSystemLibrary.K2_SetTimer` null "active trap" 1.0 true -1.0))))

(event `active trap`
  (`/Engine/EditorBlueprintResources/StandardMacros.DoOnce` false :!label _label
    (:`Completed`
      (bind (_direction _newtrack_0) (`Timeline|swing` :!label _label_2)
        (:`Update`
          (`SceneComponent.K2_SetRelativeRotation` (`self.StaticMesh2`) (`KismetMathLibrary.RLerp` (struct :`Pitch` 70.0 :`Yaw` 90.0 :`Roll` 180.0) (struct :`Pitch` -70.0 :`Yaw` 90.0 :`Roll` 180.0) _newtrack_0) false false)
          (`SceneComponent.K2_SetRelativeRotation` (`self.StaticMesh`) (`KismetMathLibrary.RLerp` (struct :`Pitch` 70.0 :`Yaw` 90.0 :`Roll` 180.0) (struct :`Pitch` -70.0 :`Yaw` 90.0 :`Roll` 180.0) _newtrack_0) false false)
          (goto _label :!via `Reset`))
        (:`Finished`
          (if (`|EnumEquality` _direction "Forward")
            (goto _label_2 :!via `Reverse`)
            (else
              (goto _label_2))))))))

(event `self.StaticMesh.OnComponentHit`
  (params (HitComponent :type "PrimitiveComponent Object Reference") (OtherActor :type "Actor Object Reference") (OtherComp :type "PrimitiveComponent Object Reference") (NormalImpulse :type "Vector Structure") (Hit :type "HitResult Structure (by ref)"))
  (bind _asbp_third_person_character (cast `/Game/ThirdPerson/Blueprints/BP_ThirdPersonCharacter` OtherActor))
  (`Character.PlayAnimMontage` _asbp_third_person_character "/Game/LabWork1/Animations/Hit_To_Body_Montage.Hit_To_Body_Montage" 1.0 "None")
  (`GameplayStatics.ApplyDamage` _asbp_third_person_character 5.0))

(event `self.StaticMesh2.OnComponentHit`
  (params (HitComponent :type "PrimitiveComponent Object Reference") (OtherActor :type "Actor Object Reference") (OtherComp :type "PrimitiveComponent Object Reference") (NormalImpulse :type "Vector Structure") (Hit :type "HitResult Structure (by ref)"))
  (bind _asbp_third_person_character (cast `/Game/ThirdPerson/Blueprints/BP_ThirdPersonCharacter` OtherActor))
  (`Character.PlayAnimMontage` _asbp_third_person_character "/Game/LabWork1/Animations/Hit_To_Body_Montage.Hit_To_Body_Montage" 1.0 "None")
  (`GameplayStatics.ApplyDamage` _asbp_third_person_character 5.0))

(fn `UserConstructionScript`)